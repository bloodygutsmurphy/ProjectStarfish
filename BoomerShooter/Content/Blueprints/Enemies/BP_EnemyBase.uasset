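; Base enemy character drawn as a multi-directional Paper2D sprite, with flipbooks chosen by facing relative to the camera.
; While recently rendered, Tick derives idle, chase, melee or ranged state from velocity and attack flags, writes it to the Blackboard, and swaps flipbooks preserving playback frame.
; RangedAttack spawns a projectile and starts a cooldown timer from a per-minute fire rate.
; Capsule overlaps trigger overlapping interactables.
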(event OnComponentBeginOverlap(CapsuleComponent)
  (params (OverlappedComponent :type Primitive%20Component%20Object%20Reference) (OtherActor :type Actor%20Object%20Reference) (OtherComp :type Primitive%20Component%20Object%20Reference) (OtherBodyIndex :type Integer) (bFromSweep :type Boolean) (SweepResult :type Hit%20Result%20Structure%20%28by%20ref%29))
  (for _array_element (Collision|GetOverlappingActors "/Game/Blueprints/Interactables/_Parent/BP_InteractableBase.BP_InteractableBase_C" :!class /Script/Engine.Actor)
    (Class|BIInteractionFunctions|OnInteracted(Message) _array_element)))

(event OnTargetPerceptionUpdated(AIPerception)
  (params (Actor :type Actor%20Object%20Reference) (Stimulus :type AI%20Stimulus%20Structure)))

(event EventTick
  (params (DeltaSeconds :type Float%20%28single-precision%29))
  (if (Class|Actor|WasRecentlyRendered 0.2)
    (CallFunction|StateMachine)
    (CallFunction|SpriteMagic (Variables|Default|GetSprite) (CallFunction|GetEnemyFlipbookArraysPerState))))

(fn ConstructionScript
  (Variables|Default|SetEnemyRateOfFire (/ 6e+01 (Variables|Default|GetEnemyRateOfFire))))

(fn SpriteMagic
  (params (Sprite :type Paper%20Flipbook%20Component%20Object%20Reference) (FlipbookArray :type Array%20of%20Paper%20Flipbook%20Object%20References))
  (bind _output_get (LocalVariables|SetLocalFlipbook (Utilities|Array|Get(acopy) FlipbookArray (CallFunction|GetFlipbookDir FlipbookArray))))
  (if (!= _output_get (Class|PaperFlipbookComponent|GetFlipbook Sprite))
    (|Assign (|TemporaryVariable) (Class|PaperFlipbookComponent|GetPlaybackPositioninFrames Sprite))
    (bind _returnvalue (Sprite|SetFlipbook (Variables|Default|GetSprite) (LocalVariables|GetLocalFlipbook)))
    (if _returnvalue
      (Class|PaperFlipbookComponent|SetPlaybackPositioninFrames (Variables|Default|GetSprite) (Math|Integer|SelectInt (|TemporaryVariable) (Class|PaperFlipbookComponent|GetFlipbookLengthinFrames Sprite) (!= (Class|PaperFlipbook|GetNumKeyFrames (LocalVariables|GetLocalFlipbook)) 0)) false)
      (return)
      (else
        (return)))
    (else
      (return))))

(fn StateMachine
  (if (> (Math|Vector|VectorLength (Transformation|GetVelocity)) 0.0)
    (Variables|Default|SetSpriteStatesNew "NewEnumerator1")
    (elif (Variables|Default|GetbCanMelee)
      (Variables|Default|SetSpriteStatesNew "NewEnumerator3")
      (elif (Variables|Default|GetbCanFire)
        (Variables|Default|SetSpriteStatesNew "NewEnumerator4")
        (else
          (Variables|Default|SetSpriteStatesNew "NewEnumerator0")))))
  (AI|Components|Blackboard|SetValueasEnum (AI|GetBlackboard 0) (Utilities|Name|MakeLiteralName "AIStates") (Variables|Default|GetSpriteStatesNew))
  (return true))

(fn RangedAttack
  (bind _projectileclass (Variables|Default|GetProjectileClass))
  (Utilities|IsValidClass _projectileclass
    (:Is%20Valid
      (bind _returnvalue (Utilities|Time|SetTimerbyFunctionName self "SetAttacking" (Variables|Default|GetEnemyRateOfFire)))
      (Variables|Default|SetEnemyFireTimer _returnvalue)
      (bind _returnvalue_2 (Game|SpawnActorfromClass _projectileclass (Transformation|GetWorldTransform (Variables|Default|GetProjectileSpawn)) "Undefined" 0 (Variables|Default|GetInitialProjectileSpeed) (Variables|Default|GetMaxProjectileSpeed) 0))
      (bind _output_get (Variables|Default|SetSpawnedProjectile _returnvalue_2))
      (Default|Init _output_get)
      (return true))
    (:Is%20Not%20Valid
      (return false))))

(fn GetEnemyFlipbookArraysPerState
  (return (Utilities|Select :Index (Variables|Default|GetSpriteStatesNew) :NewEnumerator0 (Variables|Default|GetEnemyIdle) :NewEnumerator1 (Variables|Default|GetEnemyChase) :NewEnumerator2 0 :NewEnumerator3 (Variables|Default|GetEnemyAttackMelee) :NewEnumerator4 (Variables|Default|GetEnemyAttackRanged) :NewEnumerator5 0)))

(fn GetFlipbookDir
  (params (FlipbookArray :type Array%20of%20Paper%20Flipbook%20Object%20References))
  (bind _returnvalue (Utilities|Array|Length FlipbookArray))
  (bind _returnvalue_2 (Transformation|GetActorRotation))
  (bind _returnvalue_3 (Game|GetPlayerCameraManager 0))
  (bind _returnvalue_4 (Transformation|GetActorLocation))
  (bind _returnvalue_5 (Math|Conversions|ToFloat(Integer) _returnvalue))
  (bind _returnvalue_6 (Camera|GetCameraLocation _returnvalue_3))
  (bind _returnvalue_7 (/ 3.6e+02 _returnvalue_5))
  (bind _returnvalue_8 (Math|Rotator|FindLookatRotation _returnvalue_6 _returnvalue_4))
  (bind _returnvalue_9 (Math|Rotator|Delta(Rotator) _returnvalue_2 _returnvalue_8))
  (bind _returnvalue_10 (Math|Float|SnapToGrid(Float) (.yaw _returnvalue_9) _returnvalue_7))
  (bind _returnvalue_11 (+ _returnvalue_10 1.8e+02))
  (bind _returnvalue_12 (/ _returnvalue_11 _returnvalue_7))
  (return (select (> _returnvalue 1) (Math|Float|Truncate (Math|Float|SelectFloat 0.0 _returnvalue_12 (> _returnvalue_12 (Math|Conversions|ToFloat(Integer) (- _returnvalue 1))))) 0)))

(fn SetCanMelee
  (Variables|Default|SetbCanMelee false)
  (return))