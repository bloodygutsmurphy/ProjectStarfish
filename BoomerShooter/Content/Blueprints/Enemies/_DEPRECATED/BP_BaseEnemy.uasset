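; Deprecated base enemy that fakes a 3D look with directional sprites and destroys itself when its health runs out.
; Each tick, the player's angle from the forward vector and side from the right vector pick one of eight Idle flipbooks and a relative rotation for PFEnemy.
; Angles under 45 degrees leave the sprite unchanged.
; Health starts at MaxHealth in the construction script and drops on AnyDamage.
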(event Game|Damage|EventAnyDamage
  (params (Damage :type Float%20%28single-precision%29) (DamageType :type Damage%20Type%20Object%20Reference) (InstigatedBy :type Controller%20Object%20Reference) (DamageCauser :type Actor%20Object%20Reference))
  (bind _output_get (Variables|Data|SetHealth (Math|Float|Clamp(Float) (- (Variables|Data|GetHealth) Damage) 0.0 (Variables|Data|GetMaxHealth))))
  (if (<= _output_get 0.0)
    (Actor|DestroyActor)))

(event EventTick
  (params (DeltaSeconds :type Float%20%28single-precision%29))
  (bind _player (CallFunction|GetPlayerBP))
  (bind _returnvalue (Transformation|GetActorLocation))
  (bind _returnvalue_2 (Transformation|GetActorLocation _player))
  (bind _returnvalue_3 (- _returnvalue_2 _returnvalue))
  (bind _returnvalue_4 (Math|Vector|Normalize _returnvalue_3))
  (bind _output_get (Variables|Default|SetDegrees (Class|KismetMathLibrary|DegAcos (Math|Vector|DotProduct (Transformation|GetActorForwardVector) _returnvalue_4))))
  (if (< (Math|Vector|DotProduct (Transformation|GetActorRightVector) _returnvalue_4) 0.0)
    (Math|Float|CompareFloat _output_get 1.8e+02
      (:>
        (Variables|Default|SetFlipbookIndex 0 :!label _label)
        (Variables|Default|SetNewRotation -9e+01))
      (:==
        (goto _label))
      (:<
        (Math|Float|CompareFloat (Variables|Default|GetDegrees) 135.0
          (:>
            (Variables|Default|SetFlipbookIndex 1 :!label _label_2)
            (Variables|Default|SetNewRotation 45.0))
          (:==
            (goto _label_2))
          (:<
            (Math|Float|CompareFloat (Variables|Default|GetDegrees) 9e+01
              (:>
                (Variables|Default|SetFlipbookIndex 2 :!label _label_3)
                (Variables|Default|SetNewRotation 1.8e+02))
              (:==
                (goto _label_3))
              (:<
                (Math|Float|CompareFloat (Variables|Default|GetDegrees) 45.0
                  (:>
                    _)
                  (:==
                    _))
                (Variables|Default|SetFlipbookIndex 3)
                (Variables|Default|SetNewRotation 135.0)))))))
    (else
      (Math|Float|CompareFloat (Variables|Default|GetDegrees) 1.8e+02
        (:>
          (Variables|Default|SetFlipbookIndex 4 :!label _label_4)
          (Variables|Default|SetNewRotation 9e+01))
        (:==
          (goto _label_4))
        (:<
          (Math|Float|CompareFloat (Variables|Default|GetDegrees) 135.0
            (:>
              (Variables|Default|SetFlipbookIndex 5 :!label _label_5)
              (Variables|Default|SetNewRotation 45.0))
            (:==
              (goto _label_5))
            (:<
              (Math|Float|CompareFloat (Variables|Default|GetDegrees) 9e+01
                (:>
                  (Variables|Default|SetFlipbookIndex 6 :!label _label_6)
                  (Variables|Default|SetNewRotation 0.0))
                (:==
                  (goto _label_6))
                (:<
                  (Math|Float|CompareFloat (Variables|Default|GetDegrees) 45.0
                    (:>
                      _)
                    (:==
                      _))
                  (Variables|Default|SetFlipbookIndex 7)
                  (Variables|Default|SetNewRotation -45.0)))))))))
  (Transformation|SetRelativeRotation (Variables|Default|GetPF_Enemy) (Math|Rotator|MakeRotator 0.0 0.0 (Variables|Default|GetNewRotation)) false false)
  (Sprite|SetFlipbook (Variables|Default|GetPF_Enemy) (Utilities|Array|Get(acopy) (Variables|Flipbooks|GetIdle) (Variables|Default|GetFlipbookIndex))))

(fn ConstructionScript
  (Variables|Data|SetHealth (Variables|Data|GetMaxHealth)))