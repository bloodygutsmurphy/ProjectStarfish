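; BP_StandardFunctions is a set of shared helper functions that return common game objects already cast to their Blueprint classes.
; The player character and controller getters cast from player index 0 to BP_FirstPersonCharacter and BP_PlayerController.
; GetWeaponBP builds on the character getter, casting its EquippedWeapon child actor to BP_WeaponBase.
; GetEnemyBP instead casts a passed-in object to BP_EnemyBase.
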(fn GetPlayerBP
  (return (.AsBP%20First%20Person%20Character (Utilities|Casting|CastToBP_FirstPersonCharacter (Game|GetPlayerCharacter 0)))))

(fn GetEnemyBP
  (params (Object :type Pawn%20Object%20Reference))
  (return (.AsBP%20Enemy%20Base (Utilities|Casting|CastToBP_EnemyBase Object))))

(fn GetWeaponBP
  (return (.AsBP%20Weapon%20Base (Utilities|Casting|CastToBP_WeaponBase (Variables|/Script/Engine.ChildActorComponent|GetChildActor (Variables|/Game/Blueprints/Player/BP_FirstPersonCharacter.BP_FirstPersonCharacter_C|GetEquippedWeapon (CallFunction|GetPlayerBP)))))))

(fn GetPlayerControllerBP
  (return (.AsBP%20Player%20Controller (Utilities|Casting|CastToBP_PlayerController (Game|GetPlayerController 0)))))