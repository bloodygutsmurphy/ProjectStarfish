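; BP_Pickup_MegaShield is a power-up pickup that overcharges the player's armour.
; It overrides the parent pickup's InteractionRangeEntered, calling the parent logic before raising the player's maximum armour and running AddShields.
; AddShields adds a fixed boost to current armour, clamped to the new maximum, then calls the player's SetShieldTimer.
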(fn ConstructionScript
  (|CallParentFunction))

(fn InteractionRangeEntered
  (|CallParentFunction)
  (Variables|/Game/Blueprints/Player/BP_FirstPersonCharacter.BP_FirstPersonCharacter_C|SetMaxArmour (CallFunction|GetPlayerBP) 2e+02)
  (CallFunction|AddShields)
  (return))

(fn AddShields
  (bind _player (CallFunction|GetPlayerBP))
  (Variables|/Game/Blueprints/Player/BP_FirstPersonCharacter.BP_FirstPersonCharacter_C|SetCurrentArmour _player (Math|Float|Clamp(Float) (+ (Variables|/Game/Blueprints/Player/BP_FirstPersonCharacter.BP_FirstPersonCharacter_C|GetCurrentArmour _player) 1e+02) 0.0 (Variables|/Game/Blueprints/Player/BP_FirstPersonCharacter.BP_FirstPersonCharacter_C|GetMaxArmour _player)))
  (Default|SetShieldTimer (CallFunction|GetPlayerBP))
  (return))