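; Base Blueprint for item pickups that are collected when their interaction range is entered.
; Each tick it copies the pitch and yaw of the player's camera to its own rotation, acting as a billboard aligned to the view.
; InteractionRangeEntered plays the pickup sound at the actor's location and destroys it, with no item effect applied here.
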(event EventTick
  (params (DeltaSeconds :type Float%20%28single-precision%29))
  (bind _player (CallFunction|GetPlayerBP))
  (bind _camera (Variables|/Game/Blueprints/Player/BP_FirstPersonCharacter.BP_FirstPersonCharacter_C|GetCamera _player))
  (bind _returnvalue (Transformation|GetWorldRotation _camera))
  (Utilities|IsValid _player
    (:Is%20Valid
      (Transformation|SetActorRotation (Math|Rotator|MakeRotator 0.0 (.pitch _returnvalue) (.yaw _returnvalue))))))

(fn ConstructionScript
  (|CallParentFunction))

(fn InteractionRangeEntered
  (Audio|PlaySoundatLocation (Variables|Default|GetPickupSound) (Transformation|GetActorLocation) "0, 0, 0" 1.0 1.0 0.0 0 0 0)
  (Actor|DestroyActor)
  (return))