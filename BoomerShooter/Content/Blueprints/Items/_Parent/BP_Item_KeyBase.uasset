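; BP_Item_KeyBase is a base Blueprint for key card pickups that the player collects by entering interaction range.
; On range entry it adds its Type gameplay tag to the player's AcquiredKeyCards container, then calls the parent's handling.
; From BeginPlay, the ItemBob timeline animates the PSPickup component by adding its vector as a world offset on each update.
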(event EventTick
  (params (DeltaSeconds :type Float%20%28single-precision%29))
  (|CallParentFunction DeltaSeconds) ; This node is disabled and will not be called.\nDrag off pins to build functionality.
)

(event EventBeginPlay
  (bind _vector (Timeline|ItemBob Play)
    (:Update
      (Transformation|AddWorldOffset (Variables|Default|GetPS_Pickup) _vector false false))))

(fn ConstructionScript
  (|CallParentFunction))

(fn InteractionRangeEntered
  (GameplayTags|AddGameplayTag (Variables|/Game/Blueprints/Player/BP_FirstPersonCharacter.BP_FirstPersonCharacter_C|GetAcquiredKeyCards (CallFunction|GetPlayerBP)) (Variables|Default|GetType) :!class /Script/GameplayTags.BlueprintGameplayTagLibrary)
  (|CallParentFunction)
  (return))