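; BP_ItemBase is the base Blueprint for pickup items, shown as sprites that turn with the player's view.
; The construction script assigns the item's sprite to PSItem.
; Each tick, while the player is valid, the actor copies the camera's pitch and yaw for a billboard effect.
; InteractionRangeEntered plays the pickup sound at the item's location and destroys the actor, with no item effect in this class.
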(event EventTick
  (params (DeltaSeconds :type Float%20%28single-precision%29))
  (bind _player (CallFunction|GetPlayerBP))
  (bind _camera (Variables|/Game/Blueprints/Player/BP_FirstPersonCharacter.BP_FirstPersonCharacter_C|GetCamera _player))
  (bind _returnvalue (Transformation|GetWorldRotation _camera))
  (Utilities|IsValid _player
    (:Is%20Valid
      (Transformation|SetActorRotation (Math|Rotator|MakeRotator 0.0 (.pitch _returnvalue) (.yaw _returnvalue))))))

(fn ConstructionScript
  (|CallParentFunction)
  (Rendering|Components|Sprite|SetSprite (Variables|Default|GetPS_Item) (Variables|Configuration|GetNewItemSprite)))

(fn InteractionRangeEntered
  (Audio|PlaySoundatLocation (Variables|Configuration|GetPickupSound) (Transformation|GetActorLocation) "0, 0, 0" 1.0 1.0 0.0 0 0 0)
  (Actor|DestroyActor)
  (return))