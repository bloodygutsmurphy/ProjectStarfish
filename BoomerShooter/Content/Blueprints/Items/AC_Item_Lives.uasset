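; Item component that grants extra lives to the player.
; AddExtraLife checks whether the player's current lives are below the maximum, then adds Amount and clamps the result between zero and MaxLives.
; It returns true when lives are added and false when the player is already at the maximum.
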(fn AddExtraLife
  (bind _player (CallFunction|GetPlayerBP))
  (bind _maxlives (Variables|/Game/Blueprints/Player/BP_FirstPersonCharacter.BP_FirstPersonCharacter_C|GetMaxLives _player))
  (if (< (Variables|/Game/Blueprints/Player/BP_FirstPersonCharacter.BP_FirstPersonCharacter_C|GetCurrentLives _player) _maxlives)
    (Variables|/Game/Blueprints/Player/BP_FirstPersonCharacter.BP_FirstPersonCharacter_C|SetCurrentLives (CallFunction|GetPlayerBP) (Math|Integer|Clamp(Integer) (+ (Variables|/Game/Blueprints/Player/BP_FirstPersonCharacter.BP_FirstPersonCharacter_C|GetCurrentLives _player) (Variables|Config|GetAmount)) 0 _maxlives))
    (return true)
    (else
      (return false))))