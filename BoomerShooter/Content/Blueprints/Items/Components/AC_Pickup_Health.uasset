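; AC_Pickup_Health is an item component that restores health to the player when a health pickup is used.
; AddHealth adds the component's Amount to the player's current health, clamped between zero and max health, then calls the player's OnHealthAmountUpdated dispatcher.
; It returns true when health is applied and false when the player is already at full health.
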(fn AddHealth
  (bind _player (CallFunction|GetPlayerBP))
  (bind _player_2 (CallFunction|GetPlayerBP))
  (bind _maxhealth (Variables|/Game/Blueprints/Player/BP_FirstPersonCharacter.BP_FirstPersonCharacter_C|GetMaxHealth _player_2))
  (if (< (Variables|/Game/Blueprints/Player/BP_FirstPersonCharacter.BP_FirstPersonCharacter_C|GetCurrentHealth _player_2) _maxhealth)
    (Variables|/Game/Blueprints/Player/BP_FirstPersonCharacter.BP_FirstPersonCharacter_C|SetCurrentHealth _player (Math|Float|Clamp(Float) (+ (Variables|/Game/Blueprints/Player/BP_FirstPersonCharacter.BP_FirstPersonCharacter_C|GetCurrentHealth _player_2) (Variables|Config|GetAmount)) 0.0 _maxhealth))
    (Default|CallOnHealthAmountUpdated _player)
    (return true)
    (else
      (return false))))