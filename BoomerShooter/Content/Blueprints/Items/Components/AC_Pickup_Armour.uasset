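; Actor component for armour pickups that adds armour to the player.
; AddArmour only acts when the player's current armour is below the maximum, adding Amount and clamping the result between zero and that maximum.
; It then fires the player's armour-updated notification and returns whether any armour was applied.
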(fn AddArmour
  (bind _player (CallFunction|GetPlayerBP))
  (bind _player_2 (CallFunction|GetPlayerBP))
  (bind _maxarmour (Variables|/Game/Blueprints/Player/BP_FirstPersonCharacter.BP_FirstPersonCharacter_C|GetMaxArmour _player_2))
  (if (< (Variables|/Game/Blueprints/Player/BP_FirstPersonCharacter.BP_FirstPersonCharacter_C|GetCurrentArmour _player_2) _maxarmour)
    (Variables|/Game/Blueprints/Player/BP_FirstPersonCharacter.BP_FirstPersonCharacter_C|SetCurrentArmour _player (Math|Float|Clamp(Float) (+ (Variables|/Game/Blueprints/Player/BP_FirstPersonCharacter.BP_FirstPersonCharacter_C|GetCurrentArmour _player_2) (Variables|Config|GetAmount)) 0.0 _maxarmour))
    (Default|CallOnArmourAmountUpdated _player)
    (return true)
    (else
      (return false))))