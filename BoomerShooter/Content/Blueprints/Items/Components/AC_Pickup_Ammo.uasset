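; Ammo pickup component that gives the player ammo of a given type.
; AddAmmo adds Amount to the player's AmmoPerType map entry for AmmoType, clamped between zero and that type's maximum.
; It then fires the player's ammo stats update and always returns true, even when the ammo is already full.
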(fn AddAmmo
  (bind _player (CallFunction|GetPlayerBP))
  (bind _ammotype (Variables|Config|GetAmmoType))
  (bind _ammopertype (Variables|/Game/Blueprints/Player/BP_FirstPersonCharacter.BP_FirstPersonCharacter_C|GetAmmoPerType _player))
  (Utilities|Map|Add _ammopertype _ammotype (Math|Integer|Clamp(Integer) (+ (.Value (Utilities|Map|Find _ammopertype _ammotype)) (Variables|Config|GetAmount)) 0 (Default|GetMaxAmmoPerType (CallFunction|GetPlayerBP) (Variables|Config|GetAmmoType))))
  (Default|CallOnAmmoStatsUpdated _player)
  (return true))