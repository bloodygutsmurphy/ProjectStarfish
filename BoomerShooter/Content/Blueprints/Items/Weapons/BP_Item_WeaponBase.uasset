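; Base weapon pickup item that gives the player its weapon when they enter interaction range.
; A timeline started on BeginPlay bobs the PSWeapon component through world offsets.
; On range entry, unless the valid current weapon equals NextWeapon, it sets the player's EquippedWeapon child actor class to WeaponClass, initializes it and calls PickUpWeapon and the parent handler.
; NextWeapon is only assigned to itself, and IsPickupClassNotEqualToSelf has its logic disabled.
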(event EventBeginPlay
  (bind _vector (Timeline|ItemBob Play)
    (:Update
      (Transformation|AddWorldOffset (Variables|Default|GetPS_Weapon) _vector false false))))

(fn ConstructionScript)

(fn IsPickupClassNotEqualtoSelf
  (params (Weapon :type BP%20Weapon%20Base%20Object%20Reference)))

(fn InteractionRangeEntered
  (bind _weapon (CallFunction|GetWeaponBP))
  (bind _weapon_2 (CallFunction|GetWeaponBP))
  (Utilities|IsValid _weapon
    (:Is%20Valid
      (if (!= _weapon (Variables|/Game/Blueprints/Player/BP_FirstPersonCharacter.BP_FirstPersonCharacter_C|GetNextWeapon (CallFunction|GetPlayerBP)))
        (Variables|/Game/Blueprints/Player/BP_FirstPersonCharacter.BP_FirstPersonCharacter_C|SetNextWeapon (CallFunction|GetPlayerBP) (Variables|/Game/Blueprints/Player/BP_FirstPersonCharacter.BP_FirstPersonCharacter_C|GetNextWeapon (CallFunction|GetPlayerBP)))
        (else
          (return))))
    (:Is%20Not%20Valid
      _))
  (ChildActorComponent|SetChildActorClass (Variables|/Game/Blueprints/Player/BP_FirstPersonCharacter.BP_FirstPersonCharacter_C|GetEquippedWeapon (CallFunction|GetPlayerBP)) (Variables|Default|GetWeaponClass))
  (Class|BIInitialisation|Init(Message) _weapon_2)
  (Default|PickUpWeapon (CallFunction|GetPlayerBP) _weapon_2)
  (|CallParentFunction)
  (return))