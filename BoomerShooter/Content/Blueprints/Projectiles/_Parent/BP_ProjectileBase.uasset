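; BP_ProjectileBase is a parent projectile Blueprint that damages whatever it hits, other than the player.
; Init calls InitProjectile, which is empty here.
; Hit stores the hit result and calls HandleHitDetection, which applies BaseDamage with the configured DamageType to the hit actor.
; Damage always credits player controller 0 as instigator, with the projectile as causer.
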(event Collision|EventHit
  (params (MyComp :type Primitive%20Component%20Object%20Reference) (Other :type Actor%20Object%20Reference) (OtherComp :type Primitive%20Component%20Object%20Reference) (bSelfMoved :type Boolean) (HitLocation :type Vector :default "0, 0, 0") (HitNormal :type Vector :default "0, 0, 0") (NormalImpulse :type Vector :default "0, 0, 0") (Hit :type Hit%20Result%20Structure%20%28by%20ref%29))
  (Variables|Default|SetHitResult Hit)
  (if (!= Other (CallFunction|GetPlayerBP))
    (CallFunction|HandleHitDetection)))

(event EventInit
  (CallFunction|InitProjectile))

(fn ConstructionScript)

(fn InitProjectile
  (return))

(fn HandleHitDetection
  (Game|Damage|ApplyDamage (.HitActor (Collision|BreakHitResult (Variables|Default|GetHitResult))) (Variables|Config|GetBaseDamage) (Game|GetPlayerController 0) self "/Script/Engine.DamageType")
  (return))