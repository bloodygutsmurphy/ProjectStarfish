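; Base weapon projectile Blueprint with a flipbook sprite, configurable speed and an explosion on hit.
; Construction applies the initial and max speeds to the projectile movement, and Tick copies the player camera's pitch and yaw to the actor, billboard style.
; On hit, it runs the parent handler, hands the sprite to the Explosion component, rescales it and plays a sound at its location.
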(event EventTick
  (params (DeltaSeconds :type Float%20%28single-precision%29))
  (bind _player (CallFunction|GetPlayerBP))
  (bind _camera (Variables|/Game/Blueprints/Player/BP_FirstPersonCharacter.BP_FirstPersonCharacter_C|GetCamera _player))
  (bind _returnvalue (Transformation|GetWorldRotation _camera))
  (Transformation|SetActorRotation (Math|Rotator|MakeRotator 0.0 (.pitch _returnvalue) (.yaw _returnvalue))))

(fn ConstructionScript
  (bind _projectilemovement (Variables|Default|GetProjectileMovement))
  (Variables|/Script/Engine.ProjectileMovementComponent|SetInitialSpeed _projectilemovement (Variables|Data|GetInitialSpeed))
  (Variables|/Script/Engine.ProjectileMovementComponent|SetMaxSpeed _projectilemovement (Variables|Data|GetMaxSpeed)))

(fn HandleHitDetection
  (|CallParentFunction)
  (Default|HandleExplosion (Variables|Default|GetExplosion) (Variables|Default|GetSprite) self)
  (Transformation|SetWorldScale3D (Variables|Default|GetSprite) (Math|Conversions|ToVector(Float) (Variables|Default|GetProjectileExplosionScale)))
  (Audio|PlaySoundatLocation (Variables|Default|GetExplosionSound) (Transformation|GetActorLocation) "0, 0, 0" 1.0 1.0 0.0 0 0 0)
  (return))