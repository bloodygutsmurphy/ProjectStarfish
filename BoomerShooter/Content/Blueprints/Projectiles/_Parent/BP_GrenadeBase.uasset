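; Base grenade projectile Blueprint that moves as a physics body and holds back hit detection until it has almost stopped horizontally.
; InitProjectile launches it by applying Velocity as an impulse to the Collision component.
; HandleHitDetection calls the parent's version only when the Collision velocity, with Z zeroed, is within a small tolerance of zero, so vertical motion is ignored.
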(fn ConstructionScript)

(fn InitProjectile
  (Physics|AddImpulse (Variables|Default|GetCollision) (Variables|Default|GetVelocity) "None" false)
  (return))

(fn HandleHitDetection
  (bind _collision (Variables|Default|GetCollision))
  (bind _returnvalue (Transformation|GetComponentVelocity _collision))
  (if (Math|Vector|Equal(Vector) (Math|Vector|MakeVector (.x _returnvalue) (.y _returnvalue) 0.0) "0, 0, 0" 0.2)
    (|CallParentFunction)
    (else
      (return))))