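; Base Blueprint for interactable objects, providing common hooks for entering interaction range, leaving it and being interacted with.
; Each event in the event graph forwards to a matching function, presumably for child Blueprints to override.
; The functions are empty stubs, with Interacted returning false by default, and the event graph ignores that result.
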(event EventOnInteracted
  (CallFunction|Interacted))

(event EventOnInteractionRangeExited
  (CallFunction|InteractionRangeExited))

(event EventOnInteractionRangeEntered
  (CallFunction|InteractionRangeEntered))

(fn ConstructionScript)

(fn InteractionRangeEntered
  (return))

(fn InteractionRangeExited
  (return))

(fn Interacted
  (return false))