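; Base interactable door that slides its mesh open when interacted with, returning false if it is already open.
; Open and close events set the open state, play a sound and run a timeline forward or in reverse, scaling its vector offset by the mesh's Z scale.
; Leaving interaction range while open starts a delayed one-shot timer, which is cleared when the reverse animation finishes.
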(event Custom|CloseDoor
  (bind _sm_doormesh (Variables|Default|GetSM_DoorMesh))
  (Variables|Default|SetbDoorOpen false)
  (Audio|PlaySoundatLocation (Variables|Default|GetDoorClose) (Transformation|GetActorLocation) "0, 0, 0" 1.0 1.0 0.0 0 0 0)
  (bind (_direction _vector) (Timeline|DoorTimeline Reverse)
    (:Update
      (Transformation|SetRelativeLocation _sm_doormesh (* _vector (* (.z (Variables|/Script/Engine.SceneComponent|GetRelativeScale3D _sm_doormesh)) 1e+02)) false false))
    (:Finished
      (if (Utilities|Enum|Equal(Enum) _direction "Backward")
        (Utilities|Time|ClearandInvalidateTimerbyHandle (Variables|Default|GetDoorTimer))))))

(event Custom|OpenDoor
  (bind _sm_doormesh (Variables|Default|GetSM_DoorMesh))
  (Variables|Default|SetbDoorOpen true)
  (Audio|PlaySoundatLocation (Variables|Default|GetDoorOpen) (Transformation|GetActorLocation) "0, 0, 0" 1.0 1.0 0.0 0 0 0)
  (bind (_direction _vector) (Timeline|DoorTimeline Play)
    (:Update
      (Transformation|SetRelativeLocation _sm_doormesh (* _vector (* (.z (Variables|/Script/Engine.SceneComponent|GetRelativeScale3D _sm_doormesh)) 1e+02)) false false))
    (:Finished
      (if (Utilities|Enum|Equal(Enum) _direction "Backward")
        (Utilities|Time|ClearandInvalidateTimerbyHandle (Variables|Default|GetDoorTimer))))))

(fn ConstructionScript)

(fn Interacted
  (if (not (Variables|Default|GetbDoorOpen))
    (CallFunction|OpenDoor)
    (return true)
    (else
      (return false))))

(fn InteractionRangeExited
  (if (Variables|Default|GetbDoorOpen)
    (bind _returnvalue (Utilities|Time|SetTimerbyEvent (EventDispatchers|CreateEvent :!event Custom|CloseDoor) 5.0))
    (Variables|Default|SetDoorTimer _returnvalue))
  (return))