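; AC_Explosion is an actor component that plays an explosion on its owner.
; HandleExplosion swaps the supplied Paper2D flipbook to a non-looping explosion animation and, if that succeeds, binds an event to its finish.
; It then plays a sound and runs a sphere object trace for pawns and another object type at the owner's location.
; The trace results are not used.
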(fn HandleExplosion
  (params (Flipbook :type Paper%20Flipbook%20Component%20Object%20Reference) (Actor :type Actor%20Object%20Reference))
  (bind _returnvalue (Components|GetOwner))
  (bind _returnvalue_2 (Transformation|GetActorLocation _returnvalue))
  (Components|Timeline|SetLooping Flipbook false)
  (bind _returnvalue_3 (Sprite|SetFlipbook Flipbook (Variables|Default|GetFlipbookExplosion)))
  (if _returnvalue_3
    (EventDispatchers|BindEventtoOnFinishedPlaying Flipbook (EventDispatchers|CreateEvent Actor :!event K2DestroyActor))
    (Audio|PlaySoundatLocation (Variables|Default|GetExplosionSound) _returnvalue_2 "0, 0, 0" 1.0 1.0 0.0 0 0 0)
    (Collision|SphereTraceForObjects _returnvalue_2 _returnvalue_2 4.5e+02 (Utilities|Array|MakeArray "ObjectTypeQuery3" "ObjectTypeQuery8") false 0 "None")
    (return)
    (else
      (return))))