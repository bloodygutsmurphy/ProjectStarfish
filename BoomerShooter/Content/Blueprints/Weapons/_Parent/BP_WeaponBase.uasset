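; Base weapon for the player, with a Paper2D flipbook sprite, per-type ammo and a fire-rate limit.
; Attack start checks player ammo, locks firing on a timer derived from rounds per minute, and calls SpawnProjectile per shot.
; SpawnProjectile is a stub returning false for children to override; success deducts ammo, plays animation and sound, and reports noise.
; Helpers supply a cone-spread spawn transform and a camera line trace.
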(event EventStopAttack
  (Protected|OnAttackStop))

(event EventStartAttack
  (Protected|OnAttackStart))

(event EventInit
  (Protected|OnInit))

(fn ConstructionScript
  (bind _fb_weapon (Variables|Default|GetFB_Weapon))
  (Variables|Data|SetRateOfFire (Protected|GetRateOfFire))
  (Variables|Config|SetbCanAttack true)
  (Components|Timeline|SetLooping _fb_weapon (Variables|Config|GetbLoopFlipbook))
  (if (not (Variables|Config|GetbLoopFlipbook))
    (Audio|Components|Audio|Stop _fb_weapon)))

(fn SpawnProjectile
  (return false))

(fn HasAmmo
  (return (>= (.Value (Utilities|Map|Find (Variables|/Game/Blueprints/Player/BP_FirstPersonCharacter.BP_FirstPersonCharacter_C|GetAmmoPerType (CallFunction|GetPlayerBP)) (Variables|Config|GetAmmoType))) (Variables|Data|GetAttackAmmoConsumption))))

(fn OnInit
  (Default|CallOnAmmoStatsUpdated (CallFunction|GetPlayerBP))
  (return))

(fn GetRateOfFire
  (return (/ 6e+01 (Variables|Data|GetRateOfFire))))

(fn TraceforObjects
  (LocalVariables|SetPlayerCamera (Variables|/Game/Blueprints/Player/BP_FirstPersonCharacter.BP_FirstPersonCharacter_C|GetCamera (CallFunction|GetPlayerBP)))
  (bind _outhit (Collision|LineTraceForObjects (Transformation|GetWorldLocation (LocalVariables|GetPlayerCamera)) (+ (Transformation|GetWorldLocation (LocalVariables|GetPlayerCamera)) (Math|Vector|Normalize (Math|Vector|GetForwardVector (LocalVariables|GetPlayerCamera)))) (Utilities|Array|MakeArray "ObjectTypeQuery1" "ObjectTypeQuery2" "ObjectTypeQuery3" "ObjectTypeQuery4" "ObjectTypeQuery5" "ObjectTypeQuery7") false (Utilities|Array|MakeArray (CallFunction|GetPlayerBP)) "ForDuration" true "(R=1.000000,G=0.000000,B=0.000000,A=1.000000)" "(R=0.000000,G=1.000000,B=0.000000,A=1.000000)" 0.0))
  (return _outhit))

(fn OnAttackStart
  (bind _player (CallFunction|GetPlayerBP))
  (bind _ammotype (Variables|Config|GetAmmoType))
  (bind _ammopertype (Variables|/Game/Blueprints/Player/BP_FirstPersonCharacter.BP_FirstPersonCharacter_C|GetAmmoPerType _player))
  ;[0.8281 1 0] Has Ammo
  (if (and (Private|HasAmmo) (Variables|Config|GetbCanAttack))
    (Sprite|SetFlipbook (Variables|Default|GetFB_Weapon) (Variables|Animations|GetPaperFlipbookAttack))
    ;[1 0 0.09375] Reset Can Attack
    (Variables|Config|SetbCanAttack false) ; Set to false to prevent overriding firerate
    (bind _returnvalue (Utilities|Time|SetTimerbyFunctionName self "SetCanAttack" (Variables|Data|GetRateOfFire)))
    (Variables|Config|SetFireTimer _returnvalue)
    (Utilities|FlowControl|Sequence
      (:then_0
        (for _index (range 1 (Variables|Data|Private|GetProjectilesPerShot))
          (bind _bsuccess (Protected|SpawnProjectile))
          (LocalVariables|SetbProjectileSpawned _bsuccess)))
      (:then_1
        (if (LocalVariables|GetbProjectileSpawned)
          ;[0 1 0.2734] Decrement Ammo
          (Utilities|Map|Add _ammopertype _ammotype (- (.Value (Utilities|Map|Find _ammopertype _ammotype)) (Variables|Data|GetAttackAmmoConsumption)))
          (Default|CallOnAmmoStatsUpdated (CallFunction|GetPlayerBP))
          ;[1 0.1406 0] Play Attack Flipbook
          (Audio|Components|Audio|Play (Variables|Default|GetFB_Weapon))
          (Audio|PlaySoundatLocation (Variables|SFX|GetFireSound) (Variables|/Script/Engine.SceneComponent|GetRelativeLocation (Variables|Default|GetProjectileSpawn)) "0, 0, 0" 1.0 1.0 0.0 0 0 0)
          (Class|AISenseHearing|ReportNoiseEvent (Transformation|GetActorLocation) 7.0 (CallFunction|GetPlayerBP) 0.0 "None")
          (return)
          (else
            (return)))))
    (elif (Math|Boolean|ANDBoolean (not (Private|HasAmmo)) (Variables|Config|GetbCanAttack) (Utilities|Time|IsValidTimerHandle (Variables|Config|GetFireTimer)))
      (Utilities|Time|ClearandInvalidateTimerbyHandle (Variables|Config|GetFireTimer))
      (return)
      (else
        (return)))))

(fn OnAttackStop
  (return))

(fn SetCanAttack
  (Variables|Config|SetbCanAttack true)
  (Sprite|SetFlipbook (Variables|Default|GetFB_Weapon) (Variables|Animations|GetPaperFlipbookIdle))
  (return))

(fn GetProjectileSpawnTransform
  (return (Math|Transform|MakeTransform (Transformation|GetWorldLocation (Variables|Default|GetProjectileSpawn)) (Math|Rotator|MakeRotfromX (Math|Random|RandomUnitVectorinConeinDegrees (Math|Vector|Normalize (Math|Vector|GetForwardVector (Transformation|GetWorldRotation (Variables|/Game/Blueprints/Player/BP_FirstPersonCharacter.BP_FirstPersonCharacter_C|GetCamera (CallFunction|GetPlayerBP))))) (Variables|Data|GetProjectileSpreadInConeHalfDegrees))) "0.200000,0.200000,0.200000")))