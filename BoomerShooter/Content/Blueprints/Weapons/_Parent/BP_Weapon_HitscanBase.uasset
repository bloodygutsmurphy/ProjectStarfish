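; Base Blueprint for hitscan weapons that overrides projectile spawning with an instant line trace.
; SpawnProjectile traces on the Visibility channel from the ProjectileSpawn component along a random direction within the spread cone, out to Range, with timed debug drawing.
; A hit applies BaseDamage of the configured DamageType, always instigated by player controller 0, and the function returns true whether it hits or misses.
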(fn ConstructionScript
  (|CallParentFunction))

(fn SpawnProjectile
  (bind _projectilespawn (Variables|Default|GetProjectileSpawn))
  (bind _returnvalue (Transformation|GetWorldLocation _projectilespawn))
  (bind (_outhit _returnvalue_2) (Collision|LineTraceByChannel _returnvalue (+ _returnvalue (* (Math|Random|RandomUnitVectorinConeinDegrees (Math|Vector|GetForwardVector (Transformation|GetWorldRotation _projectilespawn)) (Variables|Default|GetProjectileSpreadInConeHalfDegrees)) (Variables|Data|GetRange))) "TraceTypeQuery1" false 0 "ForDuration"))
  (if _returnvalue_2
    (Game|Damage|ApplyDamage (.HitActor (Collision|BreakHitResult _outhit)) (Variables|Default|GetBaseDamage) (Game|GetPlayerController 0) self "/Script/Engine.DamageType")
    (return true)
    (else
      (return true))))