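; Parent weapon Blueprint for full-auto projectile weapons, adding repeat fire while the attack is held.
; Attack start sets an AutoFiring flag before running the parent attack, and attack stop clears it.
; The SetCanAttack override runs the parent logic, then either starts another attack while the flag is set or clears and invalidates the FireTimer handle.
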(fn ConstructionScript
  (|CallParentFunction))

(fn OnAttackStart
  (Variables|Default|SetbAutoFiring true)
  (|CallParentFunction)
  (return))

(fn OnAttackStop
  (Variables|Default|SetbAutoFiring false)
  (return))

(fn SetCanAttack
  (|CallParentFunction)
  (if (Variables|Default|GetbAutoFiring)
    (CallFunction|StartAttack)
    (else
      (Utilities|Time|ClearandInvalidateTimerbyHandle (Variables|Default|GetFireTimer))))
  (return))