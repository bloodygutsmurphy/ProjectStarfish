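; Base Blueprint for projectile-firing weapons, supplying the shared logic that spawns a weapon's projectile.
; SpawnProjectile validates the projectile class, spawns it at the transform from GetProjectileSpawnTransform with initial and max speeds, then stores and initializes it.
; It returns whether the class was valid; the event graph and construction script add no logic of their own.
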(event EventBeginPlay)

(event Collision|EventActorBeginOverlap
  (params (OtherActor :type Actor%20Object%20Reference)))

(event EventTick
  (params (DeltaSeconds :type Float%20%28single-precision%29))
  (|CallParentFunction DeltaSeconds) ; This node is disabled and will not be called.\nDrag off pins to build functionality.
)

(fn ConstructionScript
  (|CallParentFunction))

(fn SpawnProjectile
  (bind _projectileclass (Variables|Default|GetProjectileClass))
  (Utilities|IsValidClass _projectileclass
    (:Is%20Valid
      (bind _returnvalue (Game|SpawnActorfromClass _projectileclass (CallFunction|GetProjectileSpawnTransform) "Undefined" 0 (Variables|Default|GetInitialProjectileSpeed) (Variables|Default|GetMaxProjectileSpeed) 0))
      (bind _output_get (Variables|Default|SetSpawnedProjectile _returnvalue))
      (Default|Init _output_get)
      (return true))
    (:Is%20Not%20Valid
      (return false))))