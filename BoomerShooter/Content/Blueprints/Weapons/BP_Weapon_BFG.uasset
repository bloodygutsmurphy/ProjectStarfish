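; BP_Weapon_BFG is a BFG weapon Blueprint that launches a previously spawned projectile held hidden and attached until release.
; ReleaseProjectile checks that the projectile is valid, sets its forward local velocity from InitialSpeed, enables movement simulation, detaches it in world space and unhides it.
; The construction script binds an event to the FBWeapon flipbook's finished-playing delegate, while OnInit only calls the parent.
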(event Custom|ReleaseProjectile
  (bind _spawnedprojectile (Variables|Default|GetSpawnedProjectile)
    (:then
      (Game|Components|ProjectileMovement|SetVelocityinLocalSpace (Variables|/Game/Blueprints/Projectiles/_Parent/BP_WeaponProjectileBase.BP_WeaponProjectileBase_C|GetProjectileMovement _spawnedprojectile) (Math|Vector|MakeVector (Variables|/Game/Blueprints/Projectiles/_Parent/BP_WeaponProjectileBase.BP_WeaponProjectileBase_C|GetInitialSpeed _spawnedprojectile) 0.0 0.0))
      (Variables|/Script/Engine.ProjectileMovementComponent|SetbSimulationEnabled (Variables|/Game/Blueprints/Projectiles/_Parent/BP_WeaponProjectileBase.BP_WeaponProjectileBase_C|GetProjectileMovement _spawnedprojectile) true)
      (Transformation|DetachFromActor _spawnedprojectile "KeepWorld" "KeepWorld" "KeepWorld")
      (Rendering|SetActorHiddenInGame _spawnedprojectile false))
    (:else)))

(fn ConstructionScript
  (|CallParentFunction)
  (EventDispatchers|BindEventtoOnFinishedPlaying (Variables|Default|GetFB_Weapon) (EventDispatchers|CreateEvent :!event Custom|ReleaseProjectile)))

(fn OnInit
  (|CallParentFunction)
  (return))